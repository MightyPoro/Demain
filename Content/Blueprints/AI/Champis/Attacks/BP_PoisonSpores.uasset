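; Poison spore cloud attack for the Champis AI that deals damage over time to the player.
; Looping timers widen the hitbox in X and Y by a multiplier, and another destroys the actor after its lifespan.
; Any hitbox overlap starts a repeating damage timer on the cached player's health component, regardless of what entered, and end overlap clears it.
; The construction script sizes the particle system from the box extent.
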(event OnComponentBeginOverlap(Hitbox)
  (params (OverlappedComponent :type Primitive%20Component%20Object%20Reference) (OtherActor :type Actor%20Object%20Reference) (OtherComp :type Primitive%20Component%20Object%20Reference) (OtherBodyIndex :type Integer) (bFromSweep :type Boolean) (SweepResult :type Hit%20Result%20Structure%20%28by%20ref%29))
  (bind _returnvalue (Utilities|Time|SetTimerbyEvent (delegate Custom|BeginDOT) (Variables|Default|GetDOTRate) true))
  (Variables|Default|SetTimerHandle _returnvalue))

(event OnComponentEndOverlap(Hitbox)
  (params (OverlappedComponent :type Primitive%20Component%20Object%20Reference) (OtherActor :type Actor%20Object%20Reference) (OtherComp :type Primitive%20Component%20Object%20Reference) (OtherBodyIndex :type Integer))
  (Utilities|Time|ClearandInvalidateTimerbyHandle (Variables|Default|GetTimerHandle)))

(event Custom|AutoDestroy
  (Actor|DestroyActor))

(event Custom|BeginDOT
  (Default|GetsHurt (Variables|/Game/Blueprints/Player/BP_Echo.BP_Echo_C|GetBPC_Health (Variables|Default|GetPlayer)) 4.0))

(event Custom|ScaleOverLife
  (bind _hitbox (Variables|Default|GetHitbox))
  (bind _scalevalue (Variables|Default|GetScaleValue))
  (bind _relativescale3d (Variables|/Script/Engine.SceneComponent|GetRelativeScale3D _hitbox))
  (Transformation|SetRelativeScale3D _hitbox (Math|Vector|MakeVector (* (.x _relativescale3d) _scalevalue) (* (.y _relativescale3d) _scalevalue) (.z _relativescale3d))))

(event EventBeginPlay
  (bind _asbp_echo (Utilities|Casting|CastToBP_Echo (Game|GetPlayerCharacter 0)))
  (Variables|Default|SetPlayer _asbp_echo)
  (Utilities|Time|SetTimerbyEvent (delegate Custom|ScaleOverLife) (Variables|Default|GetScaleRate) true)
  (Utilities|Time|SetTimerbyEvent (delegate Custom|AutoDestroy) (Variables|Default|GetSporesLifespan)))

(event Collision|EventActorBeginOverlap
  (params (OtherActor :type Actor%20Object%20Reference)))

(event EventTick
  (params (DeltaSeconds :type Float%20%28single-precision%29)))

(fn ConstructionScript
  (Transformation|SetRelativeScale3D (Variables|Default|GetParticleSystem) (/ (Variables|/Script/Engine.BoxComponent|GetBoxExtent (Variables|Default|GetHitbox)) 128.0)))