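; BP_SapBullet is a sap projectile for a Champis AI attack that leaves a puddle where it lands.
; The construction script randomly offsets the ProjectileMovement velocity on each axis, always adding upward lift, so shots scatter.
; When the Hitbox hits something other than a sap bullet, it spawns BP_SapPuddle at the impact point, rotated from the surface normal, passes on the instigator and destroys itself.
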(event OnComponentHit(Hitbox)
  (params (HitComponent :type Primitive%20Component%20Object%20Reference) (OtherActor :type Actor%20Object%20Reference) (OtherComp :type Primitive%20Component%20Object%20Reference) (NormalImpulse :type Vector :default "0, 0, 0") (Hit :type Hit%20Result%20Structure%20%28by%20ref%29))
  (bind _returnvalue (Math|Float|MakeLiteralFloat 1.0))
  (if (!= (.hitactor Hit) "BP_SapBullet")
    (Game|SpawnActorfromClass "/Game/Blueprints/AI/Champis/Attacks/BP_SapPuddle.BP_SapPuddle_C" (Math|Transform|MakeTransform (.impactpoint Hit) (* (Math|Conversions|RotationFromXVector (.normal Hit)) 9e+01) (Math|Vector|MakeVector _returnvalue _returnvalue _returnvalue)) "AdjustIfPossibleButAlwaysSpawn" 0 (Game|GetInstigator))
    (Actor|DestroyActor)))

(event EventBeginPlay)

(event Collision|EventActorBeginOverlap
  (params (OtherActor :type Actor%20Object%20Reference)))

(event EventTick
  (params (DeltaSeconds :type Float%20%28single-precision%29)))

(fn ConstructionScript
  (bind _projectilemovement (Variables|Default|GetProjectileMovement))
  (Variables|/Script/Engine.MovementComponent|SetVelocity _projectilemovement (Math|Vector|MakeVector (+ (.x (Variables|/Script/Engine.MovementComponent|GetVelocity _projectilemovement)) (Math|Random|RandomFloatinRange -1e+02 1e+02)) (+ (.y (Variables|/Script/Engine.MovementComponent|GetVelocity _projectilemovement)) (Math|Random|RandomFloatinRange -1e+02 1e+02)) (+ (.z (Variables|/Script/Engine.MovementComponent|GetVelocity _projectilemovement)) (Math|Random|RandomFloatinRange 5e+01 1e+02)))))