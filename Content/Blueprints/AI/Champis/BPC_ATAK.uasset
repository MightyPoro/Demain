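; BPC_ATAK is an attack component for BP_BaseChampi characters, caching its owning champi on BeginPlay.
; SimpleHit sphere-traces forward from just ahead of the champi's capsule, using configurable range, radius and debug drawing.
; On a hit, it passes AtkDamage to the target's BPC_HealthStatus via GetsHurt.
; It also replaces the ignore list with that target, so the next trace skips it.
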(event EventBeginPlay
  (bind _ascharacter (Utilities|Casting|CastToCharacter (Components|GetOwner)))
  (bind _output_get (Variables|Default|SetOwner _ascharacter))
  (bind _asbp_base_champi (Utilities|Casting|CastToBP_BaseChampi _output_get))
  (Variables|Default|SetmyChampi _asbp_base_champi))

(event EventTick
  (params (DeltaSeconds :type Float%20%28single-precision%29)))

(fn SimpleHit
  (bind _mychampi (Variables|Default|GetmyChampi))
  (bind _capsulecomponent (Variables|/Script/Engine.Character|GetCapsuleComponent _mychampi))
  (bind _returnvalue (Transformation|GetWorldLocation _capsulecomponent))
  (bind _returnvalue_2 (Math|Vector|GetForwardVector _capsulecomponent))
  (bind _returnvalue_3 (+ _returnvalue _returnvalue_2))
  (bind (_outhit _returnvalue_4) (Collision|SphereTraceByChannel _returnvalue_3 (+ _returnvalue_3 (* _returnvalue_2 (Variables|Default|GetRange))) (Variables|Default|GetRadius) "TraceTypeQuery3" false (Variables|Default|GetActorsToIgnore) (Variables|Default|GetDrawDebugType) true "(R=1.000000,G=0.000000,B=0.000000,A=1.000000)" "(R=0.000000,G=1.000000,B=0.000000,A=1.000000)" 1.0))
  (if _returnvalue_4
    (Variables|Default|SetActorsToIgnore (Utilities|Array|MakeArray (.HitActor (Collision|BreakHitResult _outhit))))
    (Default|GetsHurt (Actor|GetComponentbyClass (.HitActor (Collision|BreakHitResult _outhit)) "/Game/Blueprints/BPComponent/BPC_HealthStatus.BPC_HealthStatus_C") (Variables|Default|GetAtkDamage))))