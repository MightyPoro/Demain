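; Base mushroom (Champi) enemy character providing attack, retreat and death events for its AI.
; Root attack montages open a follow-up AOE attack through a notify and blackboard flag, while poison spores spawn with an animation.
; The retreat check fires a random burst of sap bullets, then sets a blackboard flag at one-third health or less.
; Death plays an animation, then notifies sap puddles it instigated and destroys itself within that loop.
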(event Custom|SapSplash
  ;[1 0.4322 0.08493] SapSplash_Atk
  (bind _output_get (Variables|Default|SetrandSapNumber (Math|Random|RandomIntegerinRange 2 5)))
  (for _index (range 0 _output_get)
    (Game|SpawnActorfromClass "/Game/Blueprints/AI/Champis/Attacks/BP_SapBullet.BP_SapBullet_C" (Transformation|GetWorldTransform (Variables|Default|GetSapSpawner)) "AdjustIfPossibleButAlwaysSpawn" 0 self)))

(event Custom|RootAttack
  ;[1 0.4322 0.08493] Root_Atk
  (Utilities|Array|Clear (Variables|Default|GetactorsToIgnore))
  (Input|SetIgnoreMoveInput (Variables|Default|GetmyAIController) false)
  (Animation|Montage|PlayMontage (Variables|Character|GetMesh) "/Game/Tech/Chara/Champi/Anim/ChampiAttack_Montage.ChampiAttack_Montage"
    (:OnCompleted
      (Input|ResetIgnoreMoveInput (Variables|Default|GetmyAIController) :!label _label))
    (:OnInterrupted
      (goto _label))
    (:OnNotifyBegin
      (switch name "None"
        (:canFollowUp
          (bind _output_get (Variables|Default|SetCanFollowUpAtk? true))
          (AI|Components|Blackboard|SetValueasBool (AI|GetBlackboard 0) (Utilities|Name|MakeLiteralName "FUPAtk") _output_get))))))

(event Custom|FollowUpAttack
  ;[1 0.4322 0.08493] FollowUp_Atk
  (Utilities|Array|Clear (Variables|Default|GetactorsToIgnore))
  (Variables|/Game/Blueprints/BPComponent/BPC_Attack.BPC_Attack_C|SetAOE? (Variables|Default|GetBPC_Attack) true)
  (Input|SetIgnoreMoveInput (Variables|Default|GetmyAIController) false)
  (Animation|Montage|PlayMontage (Variables|Character|GetMesh) "/Game/Tech/Chara/Champi/Anim/ChampiAttack_Montage.ChampiAttack_Montage"
    (:OnCompleted
      _)
    (:OnInterrupted
      _))
  (Input|ResetIgnoreMoveInput (Variables|Default|GetmyAIController))
  (bind _output_get (Variables|Default|SetCanFollowUpAtk? false))
  (AI|Components|Blackboard|SetValueasBool (AI|GetBlackboard 0) (Utilities|Name|MakeLiteralName "FUPAtk") _output_get)
  (Variables|/Game/Blueprints/BPComponent/BPC_Attack.BPC_Attack_C|SetAOE? (Variables|Default|GetBPC_Attack) false))

(event Custom|SpawnPoisonSpores
  ;[1 0.4322 0.08493] PoisonSpores_Atk
  (Variables|/Script/Engine.CharacterMovementComponent|SetMaxWalkSpeed (Variables|Character|GetCharacterMovement) (/ (Variables|Default|GetDefaultWalkSpeed) 5.0))
  (Utilities|FlowControl|Sequence
    (:then_0
      (Utilities|FlowControl|DoOnce false :!label _label
        (:Completed
          (Components|Animation|PlayAnimation (Variables|Character|GetMesh) "/Game/Tech/Chara/Champi/Anim/ChampiSpore.ChampiSpore" false)
          (Utilities|FlowControl|Delay 3.0)
          (goto _label Reset))))
    (:then_1
      (Game|SpawnActorfromClass "/Game/Blueprints/AI/Champis/Attacks/BP_PoisonSpores.BP_PoisonSpores_C" (Transformation|GetActorTransform) "Undefined" 0 0)
      (Variables|/Script/Engine.CharacterMovementComponent|SetMaxWalkSpeed (Variables|Character|GetCharacterMovement) (Variables|Default|GetDefaultWalkSpeed)))))

(event Custom|DoIRetreat?
  (bind _bpc_healthstatus (Variables|Default|GetBPC_HealthStatus))
  ;[1 0.4322 0.08493] REtrAZETA T
  (CallFunction|SapSplash)
  (if (<= (Variables|/Game/Blueprints/BPComponent/BPC_HealthStatus.BPC_HealthStatus_C|GetHealth _bpc_healthstatus) (/ (Variables|/Game/Blueprints/BPComponent/BPC_HealthStatus.BPC_HealthStatus_C|GetMaxHealth _bpc_healthstatus) 3.0))
    (Development|PrintString "AAAAAAAAAAAAAAAAAAAAAAAAAAAAAAAA" true true "(R=1.000000,G=0.000000,B=0.010267,A=1.000000)")
    (AI|Components|Blackboard|SetValueasBool (AI|GetBlackboard 0) (Utilities|Name|MakeLiteralName "GMalJeKour") true)
    (else
      (Development|PrintString "LetsParty"))))

(event Custom|ChampiAnimDamage
  (Animation|Montage|PlayMontage (Variables|Character|GetMesh) "/Game/Tech/Chara/Champi/Anim/Champi_Damage_Montage.Champi_Damage_Montage"))

(event EventDeath
  (Collision|SetCollisionEnabled (Variables|Collision|GetCapsuleComponent) "NoCollision")
  (Components|Animation|PlayAnimation (Variables|Character|GetMesh) "/Game/Tech/Chara/Champi/Anim/ChampiMort.ChampiMort" false)
  (Utilities|FlowControl|Delay 5.0)
  (bind _outactors (Actor|GetAllActorsOfClass "/Game/Blueprints/AI/Champis/Attacks/BP_SapPuddle.BP_SapPuddle_C"))
  (for _array_element _outactors
    (if (== (Variables|/Script/Engine.Actor|GetInstigator _array_element) self)
      (if (Utilities|DoesObjectImplementInterface _array_element "/Game/Blueprints/AI/BPI_DeathEvent.BPI_DeathEvent_C")
        (Class|BPIDeathEvent|Death(Message) _array_element)
        (Actor|DestroyActor)))))

(event Collision|EventActorBeginOverlap
  (params (OtherActor :type Actor%20Object%20Reference)))

(event EventBeginPlay
  (Variables|Default|SetmyAIController (AI|GetAIController self))
  (Variables|Default|SetDefaultWalkSpeed (Variables|/Script/Engine.CharacterMovementComponent|GetMaxWalkSpeed (Variables|Character|GetCharacterMovement)))
  (bind _asbp_echo (Utilities|Casting|CastToBP_Echo (Game|GetPlayerCharacter 0)))
  (Variables|Default|SetPlayer _asbp_echo))

(fn ConstructionScript)

(fn CalculateRunawayLoc)