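; Attack component for champion characters that deals damage to a target through a sphere trace.
; On BeginPlay it caches the owning Character and its BP_BaseChampi cast.
; SimpleHit sweeps forward from the capsule by the attack range, or in AOE mode traces a stationary sphere around the owner.
; The single hit actor receives damage through its BPC_HealthStatus and becomes the ignore list for the next trace.
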(event EventBeginPlay
  (bind _ascharacter (Utilities|Casting|CastToCharacter (Components|GetOwner)))
  (bind _output_get (Variables|Default|SetOwner _ascharacter))
  (bind _asbp_base_champi (Utilities|Casting|CastToBP_BaseChampi _output_get))
  (Variables|Default|SetmyChampi _asbp_base_champi))

(event EventTick
  (params (DeltaSeconds :type Float%20%28single-precision%29)))

(fn SimpleHit
  (bind _owner (Variables|Default|GetOwner))
  (bind _aoe_ (Variables|Default|GetAOE?))
  (bind _capsulecomponent (Variables|/Script/Engine.Character|GetCapsuleComponent _owner))
  (bind _returnvalue (Transformation|GetWorldLocation _capsulecomponent))
  (bind _returnvalue_2 (Math|Vector|GetForwardVector _capsulecomponent))
  (bind _returnvalue_3 (+ _returnvalue _returnvalue_2))
  (bind (_outhit _returnvalue_4) (Collision|SphereTraceByChannel (select _aoe_ _returnvalue _returnvalue_3) (select _aoe_ _returnvalue (+ _returnvalue_3 (* _returnvalue_2 (Variables|Default|GetAttackRange)))) (select _aoe_ (Variables|Default|GetAOERadius) (Variables|Default|GetAttackRadius)) "TraceTypeQuery3" false (Variables|Default|GetActorsToIgnore) (Variables|Default|GetDrawDebugType) true "(R=1.000000,G=0.000000,B=0.000000,A=1.000000)" "(R=0.000000,G=1.000000,B=0.000000,A=1.000000)" 1.0))
  (if _returnvalue_4
    (Variables|Default|SetActorsToIgnore (Utilities|Array|MakeArray (.HitActor (Collision|BreakHitResult _outhit))))
    (Default|GetsHurt (Actor|GetComponentbyClass (.HitActor (Collision|BreakHitResult _outhit)) "/Game/Blueprints/BPComponent/BPC_HealthStatus.BPC_HealthStatus_C") (Variables|Default|GetAtkDamage))))