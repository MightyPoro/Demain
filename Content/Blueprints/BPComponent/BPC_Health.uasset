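; Health component that tracks hit points for its owning actor and reports that actor's death to the game mode.
; TakeDamage subtracts the damage from Health, prints a debug message with the owner's name and remaining HP, and calls Deathx at zero or below.
; Deathx casts the game mode to DemainGameMode and calls GameOver with the owner.
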(event EventBeginPlay)

(event EventTick
  (params (DeltaSeconds :type Float%20%28single-precision%29)))

(fn TakeDamage
  (params (Damage :type Float%20%28single-precision%29))
  (bind _output_get (Variables|Health|SetHealth (- (Variables|Health|GetHealth) Damage)))
  (Development|PrintString (Utilities|String|Append (Utilities|GetDisplayName (Components|GetOwner)) " take " (Utilities|String|ToString(Float) Damage) " damage and has " (Utilities|String|ToString(Float) _output_get) " hp left "))
  (if (<= (Variables|Health|GetHealth) 0.0)
    (CallFunction|Death:x)))

(fn Death:x
  (bind _asdemain_game_mode (Utilities|Casting|CastToDemainGameMode (Game|GetGameMode)))
  (Default|GameOver _asdemain_game_mode (Components|GetOwner)))