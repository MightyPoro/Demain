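; Actor component that tracks an actor's health and handles taking damage, healing and death.
; GetsHurt subtracts damage, prints a debug message and, when the owner is a BP_Echo, calls its GetHurt reaction.
; At zero health or below, it reports the owner to DemainGameMode's GameOver.
; GetsHealed adds health back, capped at MaxHealth.
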(event EventBeginPlay)

(event EventTick
  (params (DeltaSeconds :type Float%20%28single-precision%29)))

(fn GetsHurt
  (params (Damage :type Float%20%28single-precision%29))
  (bind _output_get (Variables|Health|SetHealth (- (Variables|Health|GetHealth) Damage)))
  (Development|PrintString (Utilities|String|Append (Utilities|GetDisplayName (Components|GetOwner)) " get hurt for " (Utilities|String|ToString(Float) Damage) " and have " (Utilities|String|ToString(Float) _output_get) " hp left "))
  (bind _asbp_echo (Utilities|Casting|CastToBP_Echo (Components|GetOwner))
    (:then
      (Default|GetHurt _asbp_echo))
    (:CastFailed
      _))
  (if (<= _output_get 0.0)
    (CallFunction|Death:x)))

(fn Death:x
  (bind _asdemain_game_mode (Utilities|Casting|CastToDemainGameMode (Game|GetGameMode)))
  (Default|GameOver _asdemain_game_mode (Components|GetOwner)))

(fn GetsHealed
  (params (HealthBack :type Float%20%28single-precision%29))
  (if (>= (+ (Variables|Health|GetHealth) HealthBack) (Variables|Default|GetMaxHealth))
    (Variables|Health|SetHealth (Variables|Default|GetMaxHealth))
    (else
      (Variables|Health|SetHealth (+ (Variables|Health|GetHealth) HealthBack)))))