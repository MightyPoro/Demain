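; BP_TDCam is a camera pawn with a CameraBoom, built to line up with the BP_Echo actor.
; On BeginPlay it finds BP_Echo and caches it as EchoRef.
; SetTDCamWorldLocAndRot moves the boom to Echo's location and rotation, has the pawn's own controller possess it, and prints a debug "Hello".
; The EventGraph's call to that function is disconnected, so it never runs there.
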(event EventBeginPlay
  (bind _returnvalue (Actor|GetActorOfClass "/Game/Blueprints/BP_Echo.BP_Echo_C"))
  (Variables|Default|SetEchoRef _returnvalue))

(fn ConstructionScript)

(fn SetTDCamWorldLocandRot
  (bind _self self)
  (bind _echoref (Variables|Default|GetEchoRef))
  (bind _returnvalue (Transformation|GetActorTransform _echoref))
  (Transformation|SetWorldLocationAndRotation (Variables|Default|GetCameraBoom) (.location _returnvalue) (.rotation _returnvalue) false false)
  (Pawn|Possess (Pawn|GetController _self) _self)
  (Development|PrintString "Hello"))