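; Turret actor that automatically attacks BP_Golem actors entering its detection sphere.
; Sphere overlaps maintain the in-range list, and entry starts two looping timers: projectile spawning and Fire.
; Fire snaps the turret toward the closest golem, draws a debug trace and damages its BPC_HealthStatus directly, independent of projectiles and trace result.
; StopFiring clears the projectile timer but is not called here; leaving the sphere only removes the actor.
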(event OnComponentBeginOverlap(Sphere)
  (params (OverlappedComponent :type Primitive%20Component%20Object%20Reference) (OtherActor :type Actor%20Object%20Reference) (OtherComp :type Primitive%20Component%20Object%20Reference) (OtherBodyIndex :type Integer) (bFromSweep :type Boolean) (SweepResult :type Hit%20Result%20Structure%20%28by%20ref%29))
  ;[0.1395 1 0.2089] Set Actor To Check
  (Utilities|Casting|CastToBP_Golem OtherActor)
  (Utilities|Array|Add (Variables|Default|GetActorsInRange) OtherActor)
  (CallFunction|StartFiring)
  (Utilities|Time|SetTimerbyEvent (delegate Custom|Fire) (Variables|Default|GetShootRate) true))

(event OnComponentEndOverlap(Sphere)
  (params (OverlappedComponent :type Primitive%20Component%20Object%20Reference) (OtherActor :type Actor%20Object%20Reference) (OtherComp :type Primitive%20Component%20Object%20Reference) (OtherBodyIndex :type Integer))
  (Utilities|Array|RemoveItem (Variables|Default|GetActorsInRange) OtherActor))

(event Custom|Fire
  (bind _distancelist (Variables|Default|GetDistanceList))
  (bind _actorsinrange (Variables|Default|GetActorsInRange))
  (bind _turret (Variables|Default|GetTurret))
  (bind _actorsinrange_2 (Variables|Default|GetActorsInRange))
  (bind _indexofminvalue (Math|Float|MinOfFloatArray _distancelist))
  (bind _returnvalue (Transformation|GetWorldLocation _turret))
  (bind _output (Utilities|Array|Get(acopy) _actorsinrange _indexofminvalue))
  (bind _returnvalue_2 (Transformation|GetActorLocation _output))
  ;[0.3465 1 0.01291] Check Actor Distance to turret
  (if (not (== (Utilities|Array|Length _actorsinrange_2) 0))
    (for (_array_element _array_index) _actorsinrange_2
      (Utilities|Array|SetArrayElem (Variables|Default|GetDistanceList) _array_index (Transformation|GetDistanceTo self _array_element) true))
    ;[0.9835 1 0.1366] Shoot at the closest one
    (Utilities|IsValid _output
      (:Is%20Valid
        (Variables|Default|SetClosestActor _output)
        (Transformation|SetWorldRotation (Variables|Default|GetTurret) (Math|Rotator|FindLookatRotation _returnvalue _returnvalue_2) false true)
        (Collision|LineTraceByChannel _returnvalue _returnvalue_2 "TraceTypeQuery1" false 0 "ForDuration")
        ;[0.3465 1 0.01291] ApplyDamage
        (Utilities|IsValid (Actor|GetComponentbyClass (Variables|Default|GetClosestActor) "/Game/Blueprints/BPComponent/BPC_HealthStatus.BPC_HealthStatus_C")
          (:Is%20Valid
            (Default|GetsHurt (Actor|GetComponentbyClass (Variables|Default|GetClosestActor) "/Game/Blueprints/BPComponent/BPC_HealthStatus.BPC_HealthStatus_C") (Variables|Default|GetDamage))))))))

(event Custom|StopFiring
  ;[1 1 1] Projectile à connecter au reste du BP
  (Utilities|Time|ClearTimerbyFunctionName 0 "FireProjectile")
  ;;[1 1 1] Tire des Projectiles de manière répétée
  (Utilities|FlowControl|DoOnce false) ; enters at Reset
)

(event Custom|StartFiring
  ;[1 1 1] Projectile à connecter au reste du BP
  ;;[1 1 1] Tire des Projectiles de manière répétée
  (Utilities|FlowControl|DoOnce false
    (:Completed
      (CallFunction|FireProjectile)
      (Utilities|Time|SetTimerbyFunctionName 0 "FireProjectile" (/ 1.0 (Variables|Default|GetProjectilePerSecond)) true))))

(event Custom|FireProjectile
  ;[1 1 1] Projectile à connecter au reste du BP
  ;;[1 1 1] Faire apparaitre un projectile au même endroit que le PorjectileSpwanPoint
  (Game|SpawnActorfromClass "/Game/Blueprints/Bp_Projectile.Bp_Projectile_C" (Transformation|GetWorldTransform (Variables|Default|GetProjectileSpawnPoint)) "Undefined" 0 0))

(event EventBeginPlay
  (Rendering|SetRenderCustomDepth (Variables|Default|GetTurret) true))

(event Collision|EventActorBeginOverlap
  (params (OtherActor :type Actor%20Object%20Reference)))

(fn ConstructionScript)