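; Day/night cycle controller that drives the game clock shown in WBP_TimeTrack and sets whether BP_Echo can collect (off at night).
; A self-calling Delay loop rotates the directional light, updates the sky sphere and advances the time.
; Sun-pitch windows play or reverse a timeline that fades sun and skylight intensity.
; The clock hour swaps streamed LightsDay and LightsNight levels, loading night lighting in the evening and day lighting by day.
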(event Custom|DayNightCycle
  (bind _returnvalue (Utilities|Time|GetWorldDeltaSeconds))
  (bind _speed (Variables|Default|Getspeed))
  (bind _lightsourceref (Variables|Default|GetlightSourceRef))
  (bind _returnvalue_2 (Transformation|GetActorRotation _lightsourceref))
  (bind _returnvalue_3 (* _returnvalue _speed))
  (bind _timespan_hours (CallFunction|TimeElapsed _returnvalue_3))
  (Utilities|FlowControl|Sequence
    (:then_0
      (Transformation|AddActorLocalRotation _lightsourceref (Math|Rotator|MakeRotator 0.0 _returnvalue_3 0.0) false false)
      (Default|UpdateSunDirection (Variables|Default|GetskySphereref))
      (Development|PrintString "Hello" true true "(R=0.000000,G=0.660000,B=1.000000,A=1.000000)" 0.0)
      (if (and (< (.pitch _returnvalue_2) 6e+01) (> (.pitch _returnvalue_2) 45.0))
        (Utilities|FlowControl|Sequence
          (:then_0
            (Utilities|FlowControl|DoOnce false :!label _label
              (:Completed
                (bind _cycletrack (Timeline|Timeline_0 Play)
                  (:Update
                    (Rendering|Components|Light|SetIntensity (Variables|/Script/Engine.Light|GetLightComponent (Variables|Default|GetlightSourceRef)) (Math|Float|Lerp 2.75 0.2 _cycletrack))
                    (Rendering|Components|Light|SetIntensity (Variables|/Script/Engine.SkyLight|GetLightComponent (Variables|Default|GetskyLightRef)) (Math|Float|Lerp 1.0 0.4 _cycletrack)))
                  (:Finished
                    (Utilities|FlowControl|Sequence
                      (:then_0
                        (goto _label Reset))
                      (:then_1
                        (goto _label_2 Reset))))))))
          (:then_1
            (Utilities|FlowControl|Delay 0.01)
            (CallFunction|DayNightCycle)))
        (elif (and (< (.pitch _returnvalue_2) 3e+01) (> (.pitch _returnvalue_2) 15.0))
          (Utilities|FlowControl|Sequence
            (:then_0
              (Utilities|FlowControl|DoOnce false :!label _label_2
                (:Completed
                  (Timeline|Timeline_0 Reverse))))
            (:then_1
              (Utilities|FlowControl|Delay 0.01 :!label _label_3)
              (CallFunction|DayNightCycle)))
          (else
            (goto _label_3)))))
    (:then_1
      (Variables|Default|GetBP_EchoRef
        (:then
          (if (and (>= _timespan_hours 17) (< _timespan_hours 21))
            (Development|PrintString "Evening" true true "(R=1.000000,G=0.524870,B=0.000000,A=1.000000)" 0.0)
            ;[0.1876 0.447 1] Sky Night
            (Game|UnloadStreamLevel(byName) "LightsDay" true)
            (Game|LoadStreamLevel(byName) "LightsNight" true)
            (elif (or (>= _timespan_hours 21) (< _timespan_hours 6))
              (Utilities|FlowControl|Sequence
                (:then_0
                  (Development|PrintString "Night" true true "(R=0.000000,G=0.000000,B=0.000000,A=1.000000)" 0.0)
                  (Variables|/Game/Blueprints/Player/BP_Echo.BP_Echo_C|SetcanCollect (Variables|Default|GetBP_EchoRef) false))
                (:then_1
                  (Utilities|FlowControl|DoOnce true :!label _label_4)))
              (else
                (Variables|/Game/Blueprints/Player/BP_Echo.BP_Echo_C|SetcanCollect (Variables|Default|GetBP_EchoRef) true)
                (Development|PrintString "Day" true true "(R=0.000000,G=1.000000,B=0.330346,A=1.000000)" 0.0)
                ;[0.1876 0.447 1] Sky day
                (Game|UnloadStreamLevel(byName) "LightsNight" true)
                (Game|LoadStreamLevel(byName) "LightsDay" true)
                (goto _label_4 Reset)))))
        (:else)))))

(event EventBeginPlay
  (bind _asbp_echo (Utilities|Casting|CastToBP_Echo (Game|GetPlayerCharacter 0)))
  (Variables|Default|SetBP_EchoRef _asbp_echo)
  (CallFunction|CanStartDayNightCycle)
  (CallFunction|DayNightCycle)
  (bind _returnvalue (UserInterface|CreateWidget "/Game/Blueprints/Widget/WBP_TimeTrack.WBP_TimeTrack_C"))
  (bind _output_get (Variables|Default|SetUI_TimeTrackRef _returnvalue))
  (UserInterface|Viewport|AddtoViewport _output_get 0)
  (bind _returnvalue_2 (Actor|GetActorOfClass "/Engine/EngineSky/BP_Sky_Sphere.BP_Sky_Sphere_C"))
  (Rendering|SetActorHiddenInGame _returnvalue_2 true))

(fn ConstructionScript)

(fn TimeElapsed
  (params (NewParam :type Float%20%28single-precision%29))
  (bind _ui_timetrackref (Variables|Default|GetUI_TimeTrackRef))
  (bind _output_get (Variables|Default|Setseconds (+ (* NewParam 2.4e+02) (Variables|Default|Getseconds))))
  (bind _output_get_2 (Variables|Default|SetTimespan (Math|Timespan|MakeTimespan 0 (Variables|Default|GetdayStartHours) (Variables|Default|GetdayStartMinutes) (Math|Float|Truncate _output_get))))
  (Utilities|IsValid _ui_timetrackref
    (:Is%20Valid
      (Variables|/Game/Blueprints/Widget/WBP_TimeTrack.WBP_TimeTrack_C|SetTime _ui_timetrackref _output_get_2)
      (return (.days (Variables|Default|GetTimespan)) (.hours (Variables|Default|GetTimespan)) (.minutes (Variables|Default|GetTimespan))))))

(fn CanStartDayNightCycle
  (bind _returnvalue (Actor|GetActorOfClass "/Script/Engine.SkyLight"))
  (bind _output_get (Variables|Default|SetskyLightRef _returnvalue))
  (bind _returnvalue_2 (Actor|GetActorOfClass "/Engine/EngineSky/BP_Sky_Sphere.BP_Sky_Sphere_C"))
  (bind _output_get_2 (Variables|Default|SetskySphereref _returnvalue_2))
  (bind _returnvalue_3 (Actor|GetActorOfClass "/Script/Engine.DirectionalLight"))
  (bind _output_get_3 (Variables|Default|SetlightSourceRef _returnvalue_3))
  (if (Math|Boolean|ANDBoolean (Utilities|IsValid _output_get) (Utilities|IsValid _output_get_2) (Utilities|IsValid _output_get_3))
    (return)))

(fn UpdateGolemCount
  (bind _outactors (Actor|GetAllActorsOfClass "/Game/Blueprints/AI/Golem/BP_Golem.BP_Golem_C"))
  (for _array_element _outactors
    (Math|Integer|IncrementInt (Variables|Default|GetNbGolemsCount)))
  (Variables|Default|SetNbGolemsLeft (Variables|Default|GetNbGolemsCount))
  (return))