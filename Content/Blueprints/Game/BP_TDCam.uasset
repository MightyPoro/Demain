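; Top-down camera rig that pans, rotates and zooms from player input, with its spring arm pitched to a set view angle on BeginPlay.
; Move axes slide the Scene component along its forward and right vectors, while rotate actions ease its yaw by a step, disabling pawn input meanwhile.
; Zoom actions play FOV timelines while held and reverse them on release.
; A helper function places the rig above EchoRef with a steep pitch and fixed arm length.
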(event EventBeginPlay
  ;[1 0.8 0.2] BeginPlay
  ;;[0 0.3 0.7] Set TD Cams view angle
  (Transformation|SetWorldRotation (Variables|Default|GetSpringArm) (Math|Rotator|MakeRotator 0.0 (Variables|Camera|GetcameraViewAngle) 0.0) false false))

(event EventTick
  (params (DeltaSeconds :type Float%20%28single-precision%29)))

(event Input|ActionEvents|InputActionCameraZoomOut
  (params (Key :type Key%20Structure :default "None"))
  (:Pressed
    (bind _newtrack_0 (Timeline|Timeline_1 Play)
      (:Update
        (Camera|SetFieldOfView (Variables|Default|GetCamera) _newtrack_0))))
  (:Released
    (Timeline|Timeline_1 Reverse)))

(event Input|ActionEvents|InputActionCameraLRot
  (params (Key :type Key%20Structure :default "None"))
  (bind _scene (Variables|Default|GetScene))
  (bind _returnvalue (Transformation|GetWorldTransform _scene))
  ;[1 0.8 0.2] TD Camera rotation
  ;;[0 0.3 0.7] Left rotation
  (:Pressed
    (Input|DisableInput (Game|Player|GetPlayerPawn 0) (Game|GetPlayerController 0))
    (Components|MoveComponentTo _scene (.location _returnvalue) (Math|Rotator|MakeRotator (.roll (.rotation _returnvalue)) (.pitch (.rotation _returnvalue)) (+ (.yaw (.rotation _returnvalue)) (Variables|Camera|GetcameraRotationValue))) true true 0.5 true)
    (Input|EnableInput (Game|Player|GetPlayerPawn 0) (Game|GetPlayerController 0))))

(event Input|ActionEvents|InputActionCameraRRot
  (params (Key :type Key%20Structure :default "None"))
  (bind _scene (Variables|Default|GetScene))
  (bind _returnvalue (Transformation|GetWorldTransform _scene))
  ;[1 0.8 0.2] TD Camera rotation
  ;;[0 0.3 0.7] Right rotation
  (:Pressed
    (Input|DisableInput (Game|Player|GetPlayerPawn 0) (Game|GetPlayerController 0))
    (Components|MoveComponentTo _scene (.location _returnvalue) (Math|Rotator|MakeRotator (.roll (.rotation _returnvalue)) (.pitch (.rotation _returnvalue)) (- (.yaw (.rotation _returnvalue)) (Variables|Camera|GetcameraRotationValue))) true true 0.5 true)
    (Input|EnableInput (Game|Player|GetPlayerPawn 0) (Game|GetPlayerController 0))))

(event Input|ActionEvents|InputActionCameraZoomIn
  (params (Key :type Key%20Structure :default "None"))
  (:Pressed
    (bind _newtrack_0 (Timeline|Timeline_0 Play)
      (:Update
        (Camera|SetFieldOfView (Variables|Default|GetCamera) _newtrack_0))))
  (:Released
    (Timeline|Timeline_0 Reverse)))

(event Input|AxisEvents|InputAxisMoveForward
  (params (AxisValue :type Float%20%28single-precision%29))
  (bind _scene (Variables|Default|GetScene))
  ;[1 0.8 0.2] TD Camera movement
  ;;[0 0.3 0.7] TD Camera vertical movement
  (Transformation|SetWorldLocation _scene (+ (Transformation|GetWorldLocation _scene) (* (* (Math|Vector|GetForwardVector (Variables|Default|GetScene)) (Variables|Camera|Getspeed)) AxisValue)) false false))

(event Input|AxisEvents|InputAxisMoveRight
  (params (AxisValue :type Float%20%28single-precision%29))
  (bind _scene (Variables|Default|GetScene))
  ;[1 0.8 0.2] TD Camera movement
  ;;[0 0.3 0.7] TD Camera horizontal movement
  (Transformation|SetWorldLocation _scene (+ (Transformation|GetWorldLocation _scene) (* (* (Math|Vector|GetRightVector (Variables|Default|GetScene)) (Variables|Camera|Getspeed)) AxisValue)) false false))

(fn ConstructionScript)

(fn SetTDCamWorldLocandRot
  (Transformation|SetWorldLocation (Variables|Default|GetScene) (+ (.location (Transformation|GetActorTransform (Variables|Default|GetEchoRef))) "0.000000, 0,300.000000") false false)
  (Transformation|SetWorldRotation (Variables|Default|GetSpringArm) "-80.000000, 0, 0" false false)
  (Variables|/Script/Engine.SpringArmComponent|SetTargetArmLength (Variables|Default|GetSpringArm) 1.5e+03))