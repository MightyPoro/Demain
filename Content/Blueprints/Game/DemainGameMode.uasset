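; Game mode that runs the day/night cycle, counts remaining golems and respawns Echo at the PlayerStart.
; A self-calling 0.01s Delay loop rotates the sun, fades lights via timeline and advances the clock shown in WBP_TimeTrack.
; Day and evening trigger the controller's camera switch.
; Once per night, clean focused cores spawn from next-zone portals, while an unclean core 0 sends Echo to GameOver, which destroys and respawns it.
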(event Custom|DayNightCycle
  (bind _returnvalue (Utilities|Time|GetWorldDeltaSeconds))
  (bind _speed (Variables|DayNightCycle|Getspeed))
  (bind _lightsourceref (Variables|DayNightCycle|GetlightSourceRef))
  (bind _returnvalue_2 (Transformation|GetActorRotation _lightsourceref))
  (bind _returnvalue_3 (* _returnvalue _speed))
  ;[0 0.3 0.7] Display day night cycle (change lighting and sun rotation)
  (bind _timespan_hours (CallFunction|TimeElapsed _returnvalue_3))
  (Utilities|FlowControl|Sequence
    (:then_0
      (Transformation|AddActorLocalRotation _lightsourceref (Math|Rotator|MakeRotator 0.0 _returnvalue_3 0.0) false false)
      (Default|UpdateSunDirection (Variables|DayNightCycle|GetskySphereref))
      (Development|PrintString (Utilities|String|ToString(Boolean) (> (.pitch _returnvalue_2) 0.0)) true true "(R=0.000000,G=0.660000,B=1.000000,A=1.000000)" 0.0)
      (if (and (< (.pitch _returnvalue_2) 6e+01) (> (.pitch _returnvalue_2) 45.0))
        (Utilities|FlowControl|Sequence
          (:then_0
            (Utilities|FlowControl|DoOnce false :!label _label
              (:Completed
                (bind _cycletrack (Timeline|Timeline_0 Play)
                  (:Update
                    (Rendering|Components|Light|SetIntensity (Variables|/Script/Engine.Light|GetLightComponent (Variables|DayNightCycle|GetlightSourceRef)) (Math|Float|Lerp 2.75 0.2 _cycletrack))
                    (Rendering|Components|Light|SetIntensity (Variables|/Script/Engine.SkyLight|GetLightComponent (Variables|DayNightCycle|GetskyLightRef)) (Math|Float|Lerp 1.0 0.4 _cycletrack)))
                  (:Finished
                    (Utilities|FlowControl|Sequence
                      (:then_0
                        (goto _label Reset))
                      (:then_1
                        (goto _label_2 Reset))))))))
          (:then_1
            (Utilities|FlowControl|Delay 0.01)
            (CallFunction|DayNightCycle)))
        (elif (and (< (.pitch _returnvalue_2) 3e+01) (> (.pitch _returnvalue_2) 15.0))
          (Utilities|FlowControl|Sequence
            (:then_0
              (Utilities|FlowControl|DoOnce false :!label _label_2
                (:Completed
                  (Timeline|Timeline_0 Reverse))))
            (:then_1
              (Utilities|FlowControl|Delay 0.01 :!label _label_3)
              (CallFunction|DayNightCycle)))
          (else
            (goto _label_3)))))
    (:then_1
      (if (and (>= _timespan_hours 17) (< _timespan_hours 21))
        (Development|PrintString "Evening" true true "(R=1.000000,G=0.524870,B=0.000000,A=1.000000)" 0.0)
        (bind _asbp_echo_controller (Utilities|Casting|CastToBP_EchoController (Game|GetPlayerController 0)))
        (Default|CallEventDCameraSwitch _asbp_echo_controller)
        (elif (or (>= _timespan_hours 21) (< _timespan_hours 6))
          (Utilities|FlowControl|Sequence
            (:then_0
              (Development|PrintString "Night" true true "(R=0.000000,G=0.000000,B=0.000000,A=1.000000)" 0.0))
            (:then_1
              (Utilities|FlowControl|DoOnce true :!label _label_4
                (:Completed
                  (Development|PrintString "Hello")
                  (bind _outactors (Actor|GetAllActorsOfClass "/Game/Blueprints/Core/BP_Core.BP_Core_C"))
                  (for _array_element _outactors
                    (if (Variables|/Game/Blueprints/Core/BP_Core.BP_Core_C|GetisClean _array_element)
                      (if (Variables|/Game/Blueprints/Core/BP_Core.BP_Core_C|GetisFocused _array_element)
                        (bind _outactors_2 (Actor|GetAllActorsOfClass "/Game/Blueprints/AI/Portal.Portal_C"))
                        (for _array_element_2 _outactors_2
                          (if (== (Variables|/Game/Blueprints/AI/Portal.Portal_C|GetZoneNb _array_element_2) (+ (Variables|/Game/Blueprints/Core/BP_Core.BP_Core_C|GetCoreNb _array_element) 1))
                            (Default|Spawn _array_element_2 (Transformation|GetActorTransform _array_element)))))
                      (elif (== (Variables|/Game/Blueprints/Core/BP_Core.BP_Core_C|GetCoreNb _array_element) 0)
                        (bind _returnvalue_4 (Actor|GetActorOfClass "/Game/Blueprints/Player/BP_Echo.BP_Echo_C"))
                        (CallFunction|GameOver _returnvalue_4))))))))
          (else
            (Development|PrintString "Day" true true "(R=0.000000,G=1.000000,B=0.330346,A=1.000000)" 0.0)
            (bind _asbp_echo_controller_2 (Utilities|Casting|CastToBP_EchoController (Game|GetPlayerController 0)))
            (Default|CallEventDCameraSwitch _asbp_echo_controller_2)
            (goto _label_4 Reset)))))))

(event Custom|GameOver
  (params (ActorToKill :type Actor%20Object%20Reference))
  (bind _respawnlocation (Variables|Default|GetRespawnLocation))
  (Actor|DestroyActor ActorToKill)
  ;[0 0.3 0.7] Update nb Golems left on the map count
  (Utilities|Casting|CastToBP_Golem ActorToKill
    (:then
      (Math|Integer|DecrementInt (Variables|Default|GetNbGolemsLeft)))
    (:CastFailed
      ;[0.3465 1 0.01291] Respawn Echo (Destroy, Spawn, Possess)
      (Utilities|Casting|CastToBP_Echo ActorToKill)
      (bind _returnvalue (Game|SpawnActorfromClass "/Game/Blueprints/Player/BP_Echo.BP_Echo_C" (Math|Transform|MakeTransform (.location _respawnlocation) (.rotation _respawnlocation) "1,1,1") "Undefined" 0 0))
      (Pawn|Possess (Game|GetPlayerController 0) _returnvalue))))

(event EventBeginPlay
  ;[0.3465 1 0.01291] Get player's respawn location
  (bind _returnvalue (Actor|GetActorOfClass "/Script/Engine.PlayerStart"))
  (Variables|Default|SetRespawnLocation (Transformation|GetActorTransform _returnvalue))
  ;[0 0.3 0.7] Get nb Golems on the map (To put where Golems are spawned, increment count after each spawn)
  (bind _outactors (Actor|GetAllActorsOfClass "/Game/Blueprints/AI/Golem/BP_Golem.BP_Golem_C"))
  (for _array_element _outactors
    (Math|Integer|IncrementInt (Variables|Default|GetNbGolemsCount)))
  (Variables|Default|SetNbGolemsLeft (Variables|Default|GetNbGolemsCount))
  ;[0 0.3 0.7] Start Day Night Cycle
  (CallFunction|CanStartDayNightCycle)
  (CallFunction|DayNightCycle)
  (bind _returnvalue_2 (UserInterface|CreateWidget "/Game/Blueprints/Widget/WBP_TimeTrack.WBP_TimeTrack_C"))
  (bind _output_get (Variables|DayNightCycle|SetUI_TimeTrackRef _returnvalue_2))
  (UserInterface|Viewport|AddtoViewport _output_get 0))

(fn ConstructionScript)

(fn TimeElapsed
  (params (DayTime :type Float%20%28single-precision%29))
  (bind _ui_timetrackref (Variables|DayNightCycle|GetUI_TimeTrackRef))
  (bind _output_get (Variables|DayNightCycle|Setseconds (+ (* DayTime 2.4e+02) (Variables|DayNightCycle|Getseconds))))
  (bind _output_get_2 (Variables|DayNightCycle|SetTimespan (Math|Timespan|MakeTimespan 0 (Variables|DayNightCycle|GetdayStartHours) (Variables|Default|GetdayStartMinutes) (Math|Float|Truncate _output_get))))
  (Utilities|IsValid _ui_timetrackref
    (:Is%20Valid
      (Variables|/Game/Blueprints/Widget/WBP_TimeTrack.WBP_TimeTrack_C|SetTime _ui_timetrackref _output_get_2)
      (return (.days (Variables|DayNightCycle|GetTimespan)) (.hours (Variables|DayNightCycle|GetTimespan)) (.minutes (Variables|DayNightCycle|GetTimespan))))))

(fn CanStartDayNightCycle
  (bind _returnvalue (Actor|GetActorOfClass "/Script/Engine.SkyLight"))
  (bind _output_get (Variables|DayNightCycle|SetskyLightRef _returnvalue))
  (bind _returnvalue_2 (Actor|GetActorOfClass "/Engine/EngineSky/BP_Sky_Sphere.BP_Sky_Sphere_C"))
  (bind _output_get_2 (Variables|DayNightCycle|SetskySphereref _returnvalue_2))
  (bind _returnvalue_3 (Actor|GetActorOfClass "/Script/Engine.DirectionalLight"))
  (bind _output_get_3 (Variables|DayNightCycle|SetlightSourceRef _returnvalue_3))
  (if (Math|Boolean|ANDBoolean (Utilities|IsValid _output_get) (Utilities|IsValid _output_get_2) (Utilities|IsValid _output_get_3))
    (return)))