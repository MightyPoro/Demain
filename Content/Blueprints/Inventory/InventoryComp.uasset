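; Inventory component that holds item slots in an array sized at BeginPlay and toggles inventory and crafting windows on the BP_EchoController HUD canvas.
; AddToInventory tops up a partial stack of the same item class or fills the first empty slot, returning whether it succeeds.
; AddToStack caps at max stack size and recursively re-adds overflow.
; SortInventory makes a single adjacent-swap pass toward descending quantity, so it does not fully sort.
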(event EventBeginPlay
  (CallFunction|PrepareInventory))

(fn ToggleInventory
  (Variables|Default|GetinventoryWindowRef
    (:then
      (Widget|RemovefromParent (Variables|Default|GetinventoryWindowRef))
      (Variables|Default|SetinventoryWindowRef 0))
    (:else
      ;[0.7 0.1 0.1] Add it to HUD WBP?
      (bind _returnvalue (UserInterface|CreateWidget "/Game/Blueprints/Widget/Inventory/WBP_InventoryWindow.WBP_InventoryWindow_C" 0 self))
      (Variables|Default|SetinventoryWindowRef _returnvalue)
      (bind _asbp_echo_controller (Utilities|Casting|CastToBP_EchoController (Game|GetPlayerController 0)))
      (bind _returnvalue_2 (Class|CanvasPanel|AddChildtoCanvas (Variables|/Game/Blueprints/Widget/Inventory/WBP_InventoryHUD.WBP_InventoryHUD_C|GetInventoryHUDCanvas (Variables|/Game/Blueprints/Player/BP_EchoController.BP_EchoController_C|GetWBP_InventoryHUDRef _asbp_echo_controller)) (Variables|Default|GetinventoryWindowRef)))
      (Class|CanvasPanelSlot|SetAutoSize _returnvalue_2 true)
      (Class|CanvasPanelSlot|SetAlignment _returnvalue_2 "(X=0.000000,Y=0.000000)")
      (Class|CanvasPanelSlot|SetAnchors _returnvalue_2 (Utilities|Struct|MakeAnchors "(X=0.500000,Y=0.500000)" "(X=0.500000,Y=0.500000)"))
      (Class|CanvasPanelSlot|SetPosition _returnvalue_2 (Variables|Default|Getposition)))))

(fn AddtoInventory
  (params (contentToAdd :type Slot%20Struct%20Structure))
  (if (.isstackable (.itemstruct contentToAdd))
    (bind _stackindex (Utilities|HasPartialStack contentToAdd)
      (:True
        (CallFunction|AddtoStack contentToAdd _stackindex)
        (Variables|Default|SetisFunSuccess true))
      (:False
        (bind _success (CallFunction|CreateStack contentToAdd :!label _label))
        (Variables|Default|SetisFunSuccess _success)))
    (else
      (goto _label)))
  (return (Variables|Default|GetisFunSuccess)))

(fn PrepareInventory
  (Utilities|Array|Resize (Variables|Default|Getinventory) (Variables|Default|GetnbSlots)))

(fn CreateStack
  (params (contentToAdd :type Slot%20Struct%20Structure))
  (bind (_array_element _array_index) (Utilities|Array|ForEachLoopwithBreak (Variables|Default|Getinventory) :!label _label)
    (:LoopBody
      (if (<= (.qte _array_element) 0)
        (LocalVariables|SethasSpace true)
        (LocalVariables|SetspaceIndex _array_index)
        (goto _label Break)))
    (:Completed
      (if (LocalVariables|GethasSpace)
        (Utilities|Array|SetArrayElem (Variables|Default|Getinventory) (LocalVariables|GetspaceIndex) contentToAdd)
        (return (LocalVariables|GethasSpace))
        (else
          (return false))))))

(fn AddtoStack
  (params (Content :type Slot%20Struct%20Structure) (SlotIndex :type Integer))
  (bind _qte (Utilities|Struct|BreakSlotStruct Content))
  (bind _inventory (Variables|Default|Getinventory))
  (bind _inventory_2 (Variables|Default|Getinventory))
  (bind _maxstacksize (Utilities|Struct|BreakItemStruct (.itemstruct Content)))
  (bind _output (Utilities|Array|Get(acopy) _inventory SlotIndex))
  (bind _output_2 (Utilities|Array|Get(acopy) _inventory_2 SlotIndex))
  ;[0 0.3 0.7] Can the items be added to another stack?
  (LocalVariables|SetCurrentQte _qte)
  (if (> (+ _qte (.qte _output)) (.maxstacksize (.itemstruct _output)))
    ;[0 0.3 0.7] Fills a stack than create another and put whatever is left in it
    (Utilities|Array|SetArrayElem (Variables|Default|Getinventory) SlotIndex (Utilities|Struct|MakeSlotStruct (.itemstruct Content) _maxstacksize))
    (CallFunction|AddtoInventory (Utilities|Struct|MakeSlotStruct (.itemstruct Content) (- (.qte Content) (- _maxstacksize (LocalVariables|GetCurrentQte)))))
    (else
      ;[0 0.3 0.7] Fills a stack
      (Utilities|Array|SetArrayElem _inventory_2 SlotIndex (Utilities|Struct|MakeSlotStruct (.itemstruct _output_2) (+ (.qte _output_2) (LocalVariables|GetCurrentQte))))))
  (return))

(fn ToggleCraftInventory
  (Variables|Default|GetcraftInventoryWindowRef
    (:then
      (Widget|RemovefromParent (Variables|Default|GetcraftInventoryWindowRef))
      (Variables|Default|SetcraftInventoryWindowRef 0))
    (:else
      (bind _returnvalue (UserInterface|CreateWidget "/Game/Blueprints/Widget/Inventory/WBP_InventoryWindowCraft.WBP_InventoryWindowCraft_C" 0 self))
      (bind _output_get (Variables|Default|SetcraftInventoryWindowRef _returnvalue))
      (bind _asbp_echo_controller (Utilities|Casting|CastToBP_EchoController (Game|GetPlayerController 0)))
      (bind _returnvalue_2 (Class|CanvasPanel|AddChildtoCanvas (Variables|/Game/Blueprints/Widget/Inventory/WBP_InventoryHUD.WBP_InventoryHUD_C|GetInventoryHUDCanvas (Variables|/Game/Blueprints/Player/BP_EchoController.BP_EchoController_C|GetWBP_InventoryHUDRef _asbp_echo_controller)) (Variables|Default|GetcraftInventoryWindowRef)))
      (Class|CanvasPanelSlot|SetAutoSize _returnvalue_2 true)
      (Class|CanvasPanelSlot|SetAlignment _returnvalue_2 "(X=0.000000,Y=0.000000)")
      (Class|CanvasPanelSlot|SetAnchors _returnvalue_2 (Utilities|Struct|MakeAnchors "(X=0.500000,Y=0.500000)" "(X=0.500000,Y=0.500000)"))
      (Class|CanvasPanelSlot|SetPosition _returnvalue_2 (Variables|Default|Getposition)))))

(fn SortInventory
  (for (_array_element _array_index) (Variables|Default|Getinventory)
    (if (< (.qte _array_element) (.qte (Utilities|Array|Get(acopy) (Variables|Default|Getinventory) (+ _array_index 1))))
      (CallFunction|SwapInventoryElmts _array_index (+ _array_index 1)))))

(fn SwapInventoryElmts
  (params (1st :type Integer) (2nd :type Integer))
  (bind _inventory (Variables|Default|Getinventory))
  (LocalVariables|Settemp (Utilities|Array|Get(acopy) _inventory 1st))
  (Utilities|Array|SetArrayElem _inventory 1st (Utilities|Array|Get(acopy) _inventory 2nd))
  (Utilities|Array|SetArrayElem (Variables|Default|Getinventory) 2nd (LocalVariables|Gettemp)))