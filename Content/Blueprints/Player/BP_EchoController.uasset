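; Player controller Blueprint for Echo that creates the HUD and toggles possession between the third-person Echo character and the TD camera pawn.
; On CameraSwitch, the incoming camera snaps to the current view, then eases to its relative origin with MoveComponentTo while input is disabled.
; Switching to TD first moves that pawn to Echo's location and yaw.
; The starting-camera selection logic is unconnected.
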(event EventBeginPlay
  ;[0 0.3 0.7] Add HUD
  (bind _returnvalue (UserInterface|CreateWidget "/Game/Blueprints/Widget/_WBP_HUD._WBP_HUD_C"))
  (bind _output_get (Variables|Default|SetWBP_HUDRef _returnvalue))
  (UserInterface|Viewport|AddtoViewport _output_get 0)
  ;[0 0.3 0.7] Get Echo and TDCam refs
  (bind _returnvalue_2 (Actor|GetActorOfClass "/Game/Blueprints/Player/BP_TDCam.BP_TDCam_C"))
  (Variables|Default|SetTDCamRef _returnvalue_2)
  (bind _returnvalue_3 (Actor|GetActorOfClass "/Game/Blueprints/Player/BP_Echo.BP_Echo_C"))
  (Variables|Default|SetEchoRef _returnvalue_3))

(event Input|ActionEvents|InputActionCameraSwitch
  (params (Key :type Key%20Structure))
  (bind _returnvalue (Game|GetPlayerCameraManager 0))
  (bind _returnvalue_2 (Game|GetPlayerCameraManager 0))
  (bind _echoref (Variables|Default|GetEchoRef))
  (bind _returnvalue_3 (Transformation|GetActorTransform _returnvalue))
  (bind _returnvalue_4 (Transformation|GetActorTransform _returnvalue_2))
  (bind _capsulecomponent (Variables|/Script/Engine.Character|GetCapsuleComponent _echoref))
  (bind _returnvalue_5 (Transformation|GetWorldRotation _capsulecomponent))
  ;[1 0.8 0.2] Camera switch
  (:Pressed
    (Utilities|IsinTD?
      (:true
        (Variables|Default|SetisInTD false)
        ;;[0 0.3 0.7] TD Camera
        (Transformation|SetWorldLocation (Variables|/Script/Engine.Actor|GetRootComponent (Variables|Default|GetTDCamRef)) (Transformation|GetActorLocation (Variables|Default|GetEchoRef)) false false)
        (Transformation|SetWorldRotation (Variables|/Script/Engine.Actor|GetRootComponent (Variables|Default|GetTDCamRef)) (Math|Rotator|MakeRotator (.roll _returnvalue_5) 0.0 (.yaw _returnvalue_5)) false false)
        (Transformation|SetWorldLocationAndRotation (Variables|/Game/Blueprints/Player/BP_TDCam.BP_TDCam_C|GetCamera (Variables|Default|GetTDCamRef)) (.location _returnvalue_3) (.rotation _returnvalue_3) false false)
        (Pawn|Possess (Game|GetPlayerController 0) (Variables|Default|GetTDCamRef))
        (Input|DisableInput (Game|Player|GetPlayerPawn 0) (Game|GetPlayerController 0))
        (Components|MoveComponentTo (Variables|/Game/Blueprints/Player/BP_TDCam.BP_TDCam_C|GetCamera (Variables|Default|GetTDCamRef)) "0, 0, 0" "0, 0, 0" true true (Variables|Default|GetCameraLerpTime) true)
        (Input|EnableInput (Game|Player|GetPlayerPawn 0) (Game|GetPlayerController 0)))
      (:false
        (Variables|Default|SetisInTD true)
        ;;[0 0.3 0.7] TPS Camera
        (Transformation|SetWorldLocationAndRotation (Variables|/Game/Blueprints/Player/BP_Echo.BP_Echo_C|GetFollowCamera (Variables|Default|GetEchoRef)) (.location _returnvalue_4) (.rotation _returnvalue_4) false false)
        (Pawn|Possess (Game|GetPlayerController 0) (Variables|Default|GetEchoRef))
        (Input|DisableInput (Game|Player|GetPlayerPawn 0) (Game|GetPlayerController 0))
        (Components|MoveComponentTo (Variables|/Game/Blueprints/Player/BP_Echo.BP_Echo_C|GetFollowCamera (Variables|Default|GetEchoRef)) "0, 0, 0" "0, 0, 0" true true (Variables|Default|GetCameraLerpTime) true)
        (Input|EnableInput (Game|Player|GetPlayerPawn 0) (Game|GetPlayerController 0))))))

(fn ConstructionScript)