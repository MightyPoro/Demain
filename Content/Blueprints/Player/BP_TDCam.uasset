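; Top-down tower-defense camera pawn that also handles turret placement.
; Axis inputs pan the Scene component, rotate inputs ease its yaw in steps with input disabled during the move, and zoom inputs play or reverse FOV timelines.
; SpawnTurret alternates between spawning a preview-material turret that follows the cursor via a looping timer and line trace, and replacing it with a real turret at that spot.
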(event Custom|MovePreview
  (bind _returnvalue (Game|GetPlayerController 0))
  (bind _turretpreviewref (Variables|Default|GetTurretPreviewRef))
  (bind (_worldlocation _worlddirection) (Game|Player|ConvertMouseLocationToWorldSpace _returnvalue))
  (bind _outhit (Collision|LineTraceByChannel _worldlocation (+ _worldlocation (* _worlddirection 1e+05)) "TraceTypeQuery1" false (Utilities|Array|MakeArray (Variables|Default|GetTurretPreviewRef)) "None"))
  (bind _output_get (Variables|Default|SetPreviewLocation (.location _outhit)))
  (Utilities|IsValid _turretpreviewref
    (:Is%20Valid
      (Transformation|SetActorLocation _turretpreviewref _output_get false true))))

(event EventBeginPlay
  ;[1 0.8 0.2] BeginPlay
  ;;[0 0.3 0.7] Set TD Cams view angle
  (Transformation|SetWorldRotation (Variables|Default|GetSpringArm) (Math|Rotator|MakeRotator 0.0 (Variables|Camera|GetcameraViewAngle) 0.0) false false))

(event Input|ActionEvents|InputActionCameraZoomOut
  (params (Key :type Key%20Structure :default "None"))
  ;[1 0.8 0.2] TD Camera Zoom In/Out
  ;;[0 0.3 0.7] Zoom Out
  (:Pressed
    (bind _newtrack_0 (Timeline|ZoomOut Play)
      (:Update
        (Camera|SetFieldOfView (Variables|Default|GetCamera) _newtrack_0))))
  (:Released
    (Timeline|ZoomOut Reverse)))

(event Input|ActionEvents|InputActionCameraLRot
  (params (Key :type Key%20Structure :default "None"))
  (bind _scene (Variables|Default|GetScene))
  (bind _returnvalue (Transformation|GetWorldTransform _scene))
  ;[1 0.8 0.2] TD Camera rotation
  ;;[0 0.3 0.7] Left rotation
  (:Pressed
    (Input|DisableInput (Game|Player|GetPlayerPawn 0) (Game|GetPlayerController 0))
    (Components|MoveComponentTo _scene (.location _returnvalue) (Math|Rotator|MakeRotator (.roll (.rotation _returnvalue)) (.pitch (.rotation _returnvalue)) (+ (.yaw (.rotation _returnvalue)) (Variables|Camera|GetcameraRotationValue))) true true 0.5 true)
    (Input|EnableInput (Game|Player|GetPlayerPawn 0) (Game|GetPlayerController 0))))

(event Input|ActionEvents|InputActionCameraRRot
  (params (Key :type Key%20Structure :default "None"))
  (bind _scene (Variables|Default|GetScene))
  (bind _returnvalue (Transformation|GetWorldTransform _scene))
  ;[1 0.8 0.2] TD Camera rotation
  ;;[0 0.3 0.7] Right rotation
  (:Pressed
    (Input|DisableInput (Game|Player|GetPlayerPawn 0) (Game|GetPlayerController 0))
    (Components|MoveComponentTo _scene (.location _returnvalue) (Math|Rotator|MakeRotator (.roll (.rotation _returnvalue)) (.pitch (.rotation _returnvalue)) (- (.yaw (.rotation _returnvalue)) (Variables|Camera|GetcameraRotationValue))) true true 0.5 true)
    (Input|EnableInput (Game|Player|GetPlayerPawn 0) (Game|GetPlayerController 0))))

(event Input|ActionEvents|InputActionSpawnTurret
  (params (Key :type Key%20Structure :default "None"))
  (:Pressed
    (Utilities|FlowControl|FlipFlop
      (:A
        (bind _returnvalue (Game|SpawnActorfromClass "/Game/Blueprints/BP_Turret.BP_Turret_C" (Math|Transform|MakeTransform (.WorldLocation (Game|Player|ConvertMouseLocationToWorldSpace (Game|GetPlayerController 0))) "0, 0, 0" "1,1,1") "Undefined" 0 0))
        (Variables|Default|SetTurretPreviewRef _returnvalue)
        (Utilities|Time|SetTimerbyEvent (delegate Custom|MovePreview) (Utilities|Time|GetWorldDeltaSeconds) true)
        ;[0.3465 1 0.01291] hmmmm
        (Rendering|Material|SetMaterial (Variables|/Game/Blueprints/BP_Turret.BP_Turret_C|GetCannon (Variables|Default|GetTurretPreviewRef)) 0 "/Game/Materials/M_Preview.M_Preview")
        (Rendering|Material|SetMaterial (Variables|/Game/Blueprints/BP_Turret.BP_Turret_C|GetTurret (Variables|Default|GetTurretPreviewRef)) 0 "/Game/Materials/M_Preview.M_Preview")
        (Rendering|Material|SetMaterial (Variables|/Game/Blueprints/BP_Turret.BP_Turret_C|Getleg1 (Variables|Default|GetTurretPreviewRef)) 0 "/Game/Materials/M_Preview.M_Preview")
        (Rendering|Material|SetMaterial (Variables|/Game/Blueprints/BP_Turret.BP_Turret_C|Getleg2 (Variables|Default|GetTurretPreviewRef)) 0 "/Game/Materials/M_Preview.M_Preview")
        (Rendering|Material|SetMaterial (Variables|/Game/Blueprints/BP_Turret.BP_Turret_C|Getleg3 (Variables|Default|GetTurretPreviewRef)) 0 "/Game/Materials/M_Preview.M_Preview")
        (Rendering|Material|SetMaterial (Variables|/Game/Blueprints/BP_Turret.BP_Turret_C|Getleg4 (Variables|Default|GetTurretPreviewRef)) 0 "/Game/Materials/M_Preview.M_Preview"))
      (:B
        (Actor|DestroyActor (Variables|Default|GetTurretPreviewRef))
        (Game|SpawnActorfromClass "/Game/Blueprints/BP_Turret.BP_Turret_C" (Math|Transform|MakeTransform (Variables|Default|GetPreviewLocation) "0, 0, 0" "1,1,1") "Undefined" 0 0)))))

(event Input|ActionEvents|InputActionCameraZoomIn
  (params (Key :type Key%20Structure :default "None"))
  ;[1 0.8 0.2] TD Camera Zoom In/Out
  ;;[0 0.3 0.7] Zoom In
  (:Pressed
    (bind _newtrack_0 (Timeline|ZoomIn Play)
      (:Update
        (Camera|SetFieldOfView (Variables|Default|GetCamera) _newtrack_0))))
  (:Released
    (Timeline|ZoomIn Reverse)))

(event Input|AxisEvents|InputAxisMoveForward
  (params (AxisValue :type Float%20%28single-precision%29))
  (bind _scene (Variables|Default|GetScene))
  ;[1 0.8 0.2] TD Camera movement
  ;;[0 0.3 0.7] TD Camera vertical movement
  (Transformation|SetWorldLocation _scene (+ (Transformation|GetWorldLocation _scene) (* (* (Math|Vector|GetForwardVector (Variables|Default|GetScene)) (Variables|Camera|Getspeed)) AxisValue)) false false))

(event Input|AxisEvents|InputAxisMoveRight
  (params (AxisValue :type Float%20%28single-precision%29))
  (bind _scene (Variables|Default|GetScene))
  ;[1 0.8 0.2] TD Camera movement
  ;;[0 0.3 0.7] TD Camera horizontal movement
  (Transformation|SetWorldLocation _scene (+ (Transformation|GetWorldLocation _scene) (* (* (Math|Vector|GetRightVector (Variables|Default|GetScene)) (Variables|Camera|Getspeed)) AxisValue)) false false))

(fn ConstructionScript)